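; BP_Chest is an interactable chest that opens and drops a random item.
; Interract calls OpenChest, where the Open timeline's OpenRotation Z value drives the Scene component's relative pitch.
; It then spawns a random item class from DropData's Drop list at SpawnObject's world location, without waiting for the animation to finish.
; The graph has no guard against repeat interaction.
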(event Custom|OpenChest
  (bind _openrotation (Timeline|Open Play)
    (:Update
      (Transformation|SetRelativeRotation (Variables|Default|GetScene) (Math|Rotator|MakeRotator 0.0 (.z _openrotation) 0.0) false false))))

(event EventInterract
  (CallFunction|OpenChest)
  (Game|SpawnActorfromClass (.OutItem (Utilities|Array|Random (Variables|/Game/Core/Chest/BP_DropData.BP_DropData_C|GetDrop (Variables|Default|GetDropData)))) (Math|Transform|MakeTransform (Transformation|GetWorldLocation (Variables|Default|GetSpawnObject)) "0, 0, 0" "1.000000,1.000000,1.000000") "Undefined" "MultiplyWithRoot" 0 0))

(fn ConstructionScript)