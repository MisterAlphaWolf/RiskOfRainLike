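; BP_TestingZone is a test trigger zone that damages the player or adds or spends their money, depending on its TypeTesting setting.
; On BeginPlay it labels its text render with the mode name and tints the cube's Color material parameter per mode.
; Box overlap casts to BP_ThirdPersonCharacter, stores it, and calls the matching TakeDamage, AddMoney or SpendMoney with the zone's amount.
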(event OnComponentBeginOverlap(Box)
  (params (OverlappedComponent :type Primitive%20Component%20Object%20Reference) (OtherActor :type Actor%20Object%20Reference) (OtherComp :type Primitive%20Component%20Object%20Reference) (OtherBodyIndex :type Integer) (bFromSweep :type Boolean) (SweepResult :type Hit%20Result%20Structure%20%28by%20ref%29))
  (bind _asbp_third_person_character (Utilities|Casting|CastToBP_ThirdPersonCharacter OtherActor))
  (Variables|Default|SetPlayer_Ref _asbp_third_person_character)
  (switch Utilities|FlowControl|Switch|SwitchonE_TypeTesting (Variables|Testing|GetType%20Testing)
    (:NewEnumerator0
      (Default|TakeDamage (Variables|Default|GetPlayer_Ref) (Variables|Default|GetDamageGive)))
    (:NewEnumerator1
      (Default|AddMoney (Variables|Default|GetPlayer_Ref) (Variables|Default|GetMoneyGive)))
    (:NewEnumerator3
      (Default|SpendMoney (Variables|Default|GetPlayer_Ref) (Variables|Default|GetMoneySpend)))))

(event EventBeginPlay
  (Rendering|Components|TextRender|SetText (Variables|Default|GetTextRender) (Utilities|Text|ToText(String) (Utilities|String|EnumtoString (Variables|Testing|GetType%20Testing))))
  (switch Utilities|FlowControl|Switch|SwitchonE_TypeTesting (Variables|Testing|GetType%20Testing)
    (:NewEnumerator0
      (Rendering|Material|SetVectorParameterValueonMaterials (Variables|Default|GetCube) "Color" "1.000000,0.000000,0.000000"))
    (:NewEnumerator1
      (Rendering|Material|SetVectorParameterValueonMaterials (Variables|Default|GetCube) "Color" "0.000000,1.000000,0.000000"))
    (:NewEnumerator3
      (Rendering|Material|SetVectorParameterValueonMaterials (Variables|Default|GetCube) "Color" "0.000000,0.500000,0.000000"))))

(fn ConstructionScript)